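; Node manager for a squad strategy game that gathers all BP_Node actors at BeginPlay and arbitrates squad moves between them.
; RequestMovement merges same-side squads, checks accessibility of empty nodes, or resolves battles by weighted counter-unit might, with ties favoring the defender.
; When the defender wins, the battle branch destroys that winner instead of the attacker.
; Status and might queries return placeholder values per node; CheckMovement is empty.
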(event `self.ReceiveBeginPlay`
  (bind _outactors (`GameplayStatics.GetAllActorsOfClass` "/Game/Blueprints/BP_Node.BP_Node_C"))
  (set `self.Nodes` _outactors))

(fn `Calculate Might`
  (params (firing :type "/Game/Blueprints/BP_Squad Object Reference") (Counter :type "/Game/Blueprints/BP_Squad Object Reference"))
  (returns (Might :type "Float (double-precision)"))
  (return (+ (* (- (`KismetMathLibrary.Conv_IntToDouble` (`/Game/Blueprints/BP_Squad.Artillery` firing)) (`KismetMathLibrary.Conv_IntToDouble` (`/Game/Blueprints/BP_Squad.Infantry` Counter))) (`self.ArtilleryStrength`)) (* (- (`KismetMathLibrary.Conv_IntToDouble` (`/Game/Blueprints/BP_Squad.Tanks` firing)) (`KismetMathLibrary.Conv_IntToDouble` (`/Game/Blueprints/BP_Squad.Artillery` Counter))) (`self.TankStrength`)) (* (- (`KismetMathLibrary.Conv_IntToDouble` (`/Game/Blueprints/BP_Squad.Infantry` firing)) (`KismetMathLibrary.Conv_IntToDouble` (`/Game/Blueprints/BP_Squad.Tanks` Counter))) (`self.InfantryStrength`)) (* (- (`KismetMathLibrary.Conv_IntToDouble` (`/Game/Blueprints/BP_Squad.Cavalry` firing)) (`KismetMathLibrary.Conv_IntToDouble` (`/Game/Blueprints/BP_Squad.Cavalry` Counter))) (`self.CavalryStrength`)))))

(fn `CheckMovement`)

(fn `Request Might Expectations`
  (returns (Response :type "Array of Float (double-precision)"))
  (bind _mightbuffer (`self.MightBuffer`))
  (`KismetArrayLibrary.Array_Clear` _mightbuffer)
  (for _ (`self.Nodes`)
    (`KismetArrayLibrary.Array_Add` _mightbuffer))
  (return _mightbuffer))

(fn `Request Node Status`
  (returns (Response :type "Array of /Game/Blueprints/TerrainStates Enum"))
  (bind _status_buffer (`self.Status Buffer`))
  (`KismetArrayLibrary.Array_Clear` _status_buffer)
  (for _ (`self.Nodes`)
    (`KismetArrayLibrary.Array_Add` _status_buffer "NewEnumerator3"))
  (return _status_buffer))

(fn `RequestMovement`
  (params (SquadRequesting :type "/Game/Blueprints/BP_Squad Object Reference") (TargetPosition :type "/Game/Blueprints/BP_Node Object Reference"))
  (returns (`Response ` :type Boolean))
  (bind _squadstationedhere (`/Game/Blueprints/BP_Node.SquadStationedHere` TargetPosition))
  (bind _side (`/Game/Blueprints/BP_Squad.Side` SquadRequesting))
  (if (`/Game/Blueprints/BP_Node.IsSquadStationed` TargetPosition)
    (if (== _side (`/Game/Blueprints/BP_Squad.Side` _squadstationedhere))
      (`/Game/Blueprints/BP_ArmyManager.MergeArmies` _side _squadstationedhere SquadRequesting)
      (else
        (bind (_survivor _loser) (`self.Simulate Battle` SquadRequesting _squadstationedhere))
        (bind _returnvalue (== _survivor SquadRequesting))
        (if _returnvalue
          (`self.K2_DestroyActor` _loser)
          (else
            (`self.K2_DestroyActor` _survivor)))
        (return _returnvalue)))
    (elif (`/Game/Blueprints/BP_Node.IsAccesible` TargetPosition)
      (return true)
      (else
        (return false)))))

(fn `Simulate Battle`
  (params (Attacker :type "/Game/Blueprints/BP_Squad Object Reference") (Defender :type "/Game/Blueprints/BP_Squad Object Reference"))
  (returns (Survivor :type "/Game/Blueprints/BP_Squad Object Reference") (Loser :type "/Game/Blueprints/BP_Squad Object Reference"))
  (bind _might (`self.Calculate Might` Attacker Defender))
  (bind _might_2 (`self.Calculate Might` Defender Attacker))
  (if (> _might _might_2)
    (return Attacker Defender)
    (else
      (return Defender Attacker))))

(fn `UserConstructionScript`)