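; BP_Squad is a squad unit that occupies and moves between linked location nodes on behalf of its Side.
; Tick runs an order timer, periodically asking the Side for a destination and passing it to MoveTo.
; MoveTo accepts only neighbouring nodes, and both it and SpawnAt need NodeManger approval before marking the target as occupied.
; Neither function clears the previous node's occupancy; MoveTo's clearing nodes are unconnected.
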(event `self.ReceiveBeginPlay`
  (`KismetSystemLibrary.PrintString` "Squad deployed and ready for action"))

(event `self.ReceiveTick`
  (params (DeltaSeconds :type "Float (single-precision)"))
  (bind _timesincelastorder (`self.TimeSinceLastOrder`))
  (set `self.TimeSinceLastOrder` (+ DeltaSeconds _timesincelastorder))
  (if (>= _timesincelastorder (`self.TimeBetweenOrders`))
    (`KismetSystemLibrary.PrintString` "Execute Order 66")
    (set `self.TimeSinceLastOrder` 0.0)
    (bind _response (`/Game/Blueprints/BP_ArmyManager.RequestDirections` (`self.Side`) (`self.Current Location`) self))
    (`self.MoveTo` _response)
    (`KismetSystemLibrary.PrintString` "Order66 Executed")))

(fn `GetNeighbours`
  (returns (Neighbours :type "Array of Actor Object Reference"))
  (return (`/Game/Blueprints/BP_Node.Neighbours` (`self.Current Location`))))

(fn `MoveTo`
  (params (`Target Location` :type "/Game/Blueprints/BP_Node Object Reference"))
  ;[1 1 1] check if the target location is accesible
  (if (`KismetArrayLibrary.Array_Contains` (`/Game/Blueprints/BP_Node.Neighbours` (`self.Current Location`)) `Target Location`)
    (bind _response_ (`/Game/Blueprints/BP_NodeManager.RequestMovement` (`self.NodeManger`) self `Target Location`))
    (if _response_
      (set `self.Current Location` `Target Location`)
      (set `/Game/Blueprints/BP_Node.IsSquadStationed` true `Target Location`)
      (set `/Game/Blueprints/BP_Node.SquadStationedHere` self `Target Location`))
    (else
      (`KismetSystemLibrary.PrintString` "Movement Failed, invalid target"))))

(fn `spawn at`
  (params (`Spawn Location` :type "/Game/Blueprints/BP_Node Object Reference"))
  (bind _response_ (`/Game/Blueprints/BP_NodeManager.RequestMovement` (`self.NodeManger`) self `Spawn Location`))
  (if _response_
    (set `self.Current Location` `Spawn Location`)
    (set `/Game/Blueprints/BP_Node.IsSquadStationed` true `Spawn Location`)
    (set `/Game/Blueprints/BP_Node.SquadStationedHere` self `Spawn Location`)))

(fn `UserConstructionScript`)