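; BP_PickupBase is a sprite-based pickup that the player drags with the mouse cursor.
; Hovering while the bunker pawn holds nothing enables custom depth highlighting and registers it as PointerObject.
; Clicking or SimulateClick sets HeldObject, and Tick sweeps it to the cursor trace's X/Z at fixed depth.
; A DoOnce, re-armed by each click, drops it with a sound when the MyMouse axis reads zero.
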(event `self.ReceiveBeginPlay`
  (set `self.MySprite` (`PaperSpriteComponent.GetSprite` (`self.Sprite`))))

(event `self.ReceiveTick`
  (params (DeltaSeconds :type "Float (single-precision)"))
  (if (`self.IsHeld`)
    (`self.K2_SetActorLocation` (`KismetMathLibrary.MakeVector` (.x (`.Location` (`GameplayStatics.BreakHitResult` (`PlayerController.GetHitResultUnderCursorByChannel` (`GameplayStatics.GetPlayerController` 0) "TraceTypeQuery1" true)))) -1000.0 (.z (`.Location` (`GameplayStatics.BreakHitResult` (`PlayerController.GetHitResultUnderCursorByChannel` (`GameplayStatics.GetPlayerController` 0) "TraceTypeQuery1" true))))) true)))

(event `self.Sprite.OnBeginCursorOver`
  (params (TouchedComponent :type "PrimitiveComponent Object Reference"))
  (`self.CheckPlayerHolding`
    (:`True`
      (`PrimitiveComponent.SetRenderCustomDepth` TouchedComponent true)
      (set `/Game/Blueprints/PlayerStuff/BP_BunkerPlayerPawn.PointerObject` self (cast `/Game/Blueprints/PlayerStuff/BP_BunkerPlayerPawn` (`Controller.K2_GetPawn` (`GameplayStatics.GetPlayerController` 0)) :!pure true)))))

(event `self.Sprite.OnEndCursorOver`
  (params (TouchedComponent :type "PrimitiveComponent Object Reference"))
  (`PrimitiveComponent.SetRenderCustomDepth` TouchedComponent false))

(event `self.Sprite.OnClicked`
  (params (TouchedComponent :type "PrimitiveComponent Object Reference") (ButtonPressed :type "Key Structure"))
  (bind _sprite (`self.Sprite`))
  (bind _asbp_bunker_player_pawn (cast `/Game/Blueprints/PlayerStuff/BP_BunkerPlayerPawn` (`Controller.K2_GetPawn` (`GameplayStatics.GetPlayerController` 0)) :!pure true))
  (`|ExecutionSequence` :!label _label
    (:`then_0`
      (set `self.IsHeld` true)
      (`PrimitiveComponent.SetCollisionResponseToChannel` _sprite "ECC_Camera" "ECR_Ignore")
      (`PaperSpriteComponent.SetSprite` _sprite "/Game/ArtAssets/Nick/SPR_TempBook2.SPR_TempBook2")
      (`PaperSpriteComponent.SetSprite` _sprite (`self.MySprite`))
      (`GameplayStatics.PlaySound2D` (`self.PickUpSound`) 1.0 (`KismetMathLibrary.RandomFloatInRange` 0.9 1.1))
      (set `/Game/Blueprints/PlayerStuff/BP_BunkerPlayerPawn.HeldObject` self _asbp_bunker_player_pawn))
    (:`then_1`
      (goto _label_2 :!via `Reset`))))

(event `SimulateClick`
  (goto _label))

(event `InputAxis|MyMouse` :consume false
  (params (AxisValue :type "Float (single-precision)"))
  (if (== AxisValue 0.0)
    (`/Engine/EditorBlueprintResources/StandardMacros.DoOnce` true :!label _label_2
      (:`Completed`
        (`PrimitiveComponent.SetCollisionResponseToChannel` (`self.Sprite`) "ECC_Camera" "ECR_Block")
        (set `self.IsHeld` false)
        (`GameplayStatics.PlaySound2D` (`self.PlaceDownSound`) 1.0 (`KismetMathLibrary.RandomFloatInRange` 0.9 1.1))
        (set `/Game/Blueprints/PlayerStuff/BP_BunkerPlayerPawn.HeldObject` null (cast `/Game/Blueprints/PlayerStuff/BP_BunkerPlayerPawn` (`Controller.K2_GetPawn` (`GameplayStatics.GetPlayerController` 0)) :!pure true))))))

(fn `UserConstructionScript`)