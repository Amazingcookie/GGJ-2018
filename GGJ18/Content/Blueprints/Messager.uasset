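; Messager actor that runs a translation task, issuing messages as BP_PunchCard actors and checking the strings it receives.
; A received string matching the current CorrectTranslation entry advances the message index and spawns a new card at its root transform.
; Receiving the untranslated Incoming string or calling Respawn spawns a card without advancing, while other strings do nothing.
; BeginPlay starts the sequence through NextMessage, so the index increments before the first card spawns.
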(event `Receive Message`
  (params (`sent String` :type String))
  (bind _current_message (`self.current message`))
  (if (`KismetStringLibrary.EqualEqual_StrStr` `sent String` (`|GetArrayItem` (`self.Correct Translation`) _current_message))
    (`self.Next Message`)
    (elif (`KismetStringLibrary.EqualEqual_StrStr` `sent String` (`|GetArrayItem` (`self.Incoming`) _current_message))
      (`|SpawnActorFromClass` "/Game/Blueprints/TableObjects/BP_PunchCard.BP_PunchCard_C" (`SceneComponent.K2_GetComponentToWorld` (`self.DefaultSceneRoot`)) "Undefined" "OverrideRootScale" null (`|GetArrayItem` (`self.Incoming`) (stale `Next Message` _result)) null :!label _label))))

(event `Next Message`
  (bind _result (`/Engine/EditorBlueprintResources/StandardMacros.IncrementInt` (`self.current message`))
    (:`  `
      (goto _label))))

(event `self.ReceiveBeginPlay`
  (`self.Next Message`))

(event `Respawn`
  (goto _label))

(fn `UserConstructionScript`)