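; BP_FreqFinder is an interactable radio-style table object for tuning a frequency and sending punch card messages.
; Clicking the Spinner starts seeking: Tick turns axis input into a clamped frequency, updating the text and sliding Cube until MyMouse releases.
; DoInteraction grabs the player's held punch card, or destroys one already stored.
; Clicking the Handle passes the card's PunchValues, without the frequency, to Messager, destroys it and plays Morse audio.
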(event `self.ReceiveTick`
  (params (DeltaSeconds :type "Float (single-precision)"))
  (`parent.ReceiveTick` DeltaSeconds)
  (if (`self.SeekingFreq`)
    (bind _output_get (set `self.frequency` (`KismetMathLibrary.Clamp` (+ (`self.frequency`) (`KismetMathLibrary.FCeil` (`self.GetInputAxisKeyValue`))) 800 1200)))
    (`TextRenderComponent.K2_SetText` (`self.freqtext`) (`KismetTextLibrary.Conv_DoubleToText` (* _output_get 0.1) "HalfToEven"))
    (`SceneComponent.K2_SetRelativeLocation` (`self.Cube`) (`KismetMathLibrary.MakeVector` (+ -400.0 (`KismetMathLibrary.Conv_IntToDouble` _output_get) -960.0) -12.0 -70.0) false true)))

(event `self.DoInteraction`
  (if (`KismetSystemLibrary.IsValid` (`self.InternalPunchCard`))
    (`self.K2_DestroyActor` (`self.InternalPunchCard`))
    (else
      (bind _output_get (set `self.InternalPunchCard` (cast `/Game/Blueprints/TableObjects/BP_PunchCard` (`/Game/Blueprints/PlayerStuff/BP_BunkerPlayerPawn.HeldObject` (cast `/Game/Blueprints/PlayerStuff/BP_BunkerPlayerPawn` (`Controller.K2_GetPawn` (`GameplayStatics.GetPlayerController` 0)) :!pure true)) :!pure true)))
      (`self.K2_SetActorRelativeLocation` _output_get (0.0 -2000.0 0.0) false true))))

(event `self.Spinner.OnBeginCursorOver`
  (params (TouchedComponent :type "PrimitiveComponent Object Reference"))
  (`PrimitiveComponent.SetRenderCustomDepth` TouchedComponent true))

(event `self.Spinner.OnEndCursorOver`
  (params (TouchedComponent :type "PrimitiveComponent Object Reference"))
  (`PrimitiveComponent.SetRenderCustomDepth` TouchedComponent false))

(event `self.Spinner.OnClicked`
  (params (TouchedComponent :type "PrimitiveComponent Object Reference") (ButtonPressed :type "Key Structure"))
  (set `self.SeekingFreq` true))

(event `InputAxis|MyMouse` :consume false
  (params (AxisValue :type "Float (single-precision)"))
  (bind _sprite (`self.Sprite`))
  (if (== AxisValue 1.0)
    (`PrimitiveComponent.SetCollisionResponseToChannel` _sprite "ECC_Camera" "ECR_Block")
    (else
      (`PrimitiveComponent.SetCollisionResponseToChannel` _sprite "ECC_Camera" "ECR_Ignore")
      (set `self.SeekingFreq` false))))

(event `self.Handle.OnBeginCursorOver`
  (params (TouchedComponent :type "PrimitiveComponent Object Reference"))
  (`PrimitiveComponent.SetRenderCustomDepth` TouchedComponent true))

(event `self.Handle.OnEndCursorOver`
  (params (TouchedComponent :type "PrimitiveComponent Object Reference"))
  (`PrimitiveComponent.SetRenderCustomDepth` TouchedComponent false))

(event `self.Handle.OnClicked`
  (params (TouchedComponent :type "PrimitiveComponent Object Reference") (ButtonPressed :type "Key Structure"))
  ;[1 1 1] Send stuff
  (`/Game/Blueprints/Messager.Receive Message` (`self.Messager`) (`/Game/Blueprints/TableObjects/BP_PunchCard.PunchValues` (`self.InternalPunchCard`)))
  (`self.K2_DestroyActor` (`self.InternalPunchCard`))
  (set `self.InternalPunchCard` null)
  (`GameplayStatics.PlaySound2D` "/Game/ArtAssets/Audio/morse_out.morse_out"))

(fn `UserConstructionScript`
  (`parent.UserConstructionScript`))