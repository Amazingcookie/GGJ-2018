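; Table machine that punches letter codes onto the punch card held by the player pawn.
; Interacting takes the held card, moves it away and shows a card sprite in its place, with its code on a text render.
; Eight sprite buttons highlight via custom depth on hover and append letters A to H, capped at eight characters.
; Clicking the card sprite returns the card to the player's hand and clears the display.
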(event `self.DoInteraction`
  (bind _output_get (set `self.InternalPunchCard` (cast `/Game/Blueprints/TableObjects/BP_PunchCard` (`/Game/Blueprints/PlayerStuff/BP_BunkerPlayerPawn.HeldObject` (cast `/Game/Blueprints/PlayerStuff/BP_BunkerPlayerPawn` (`Controller.K2_GetPawn` (`GameplayStatics.GetPlayerController` 0)) :!pure true)) :!pure true)))
  (`TextRenderComponent.K2_SetText` (`self.TextRender`) (`KismetTextLibrary.Conv_StringToText` (`/Game/Blueprints/TableObjects/BP_PunchCard.PunchValues` _output_get)))
  (`self.K2_SetActorRelativeLocation` _output_get (0.0 -2000.0 0.0) false true)
  (`SceneComponent.SetVisibility` (`self.PunchCardSPR`) true false))

(event `self.SPR_buttonmask1.OnBeginCursorOver`
  (params (TouchedComponent :type "PrimitiveComponent Object Reference"))
  (`PrimitiveComponent.SetRenderCustomDepth` TouchedComponent true))

(event `self.SPR_buttonmask1.OnClicked`
  (params (TouchedComponent :type "PrimitiveComponent Object Reference") (ButtonPressed :type "Key Structure"))
  (bind _internalpunchcard (`self.InternalPunchCard`))
  (bind _internalpunchcard_2 (`self.InternalPunchCard`))
  (if (and (`KismetSystemLibrary.IsValid` _internalpunchcard) (< (`KismetStringLibrary.Len` (`/Game/Blueprints/TableObjects/BP_PunchCard.PunchValues` _internalpunchcard)) 8))
    (set `self.LastCharacter` "A")
    (bind _output_get (set `/Game/Blueprints/TableObjects/BP_PunchCard.PunchValues` (`KismetStringLibrary.Concat_StrStr` (`/Game/Blueprints/TableObjects/BP_PunchCard.PunchValues` _internalpunchcard_2) (`self.LastCharacter`)) _internalpunchcard_2 :!label _label))
    (`TextRenderComponent.K2_SetText` (`self.TextRender`) (`KismetTextLibrary.Conv_StringToText` _output_get))))

(event `self.SPR_buttonmask1.OnEndCursorOver`
  (params (TouchedComponent :type "PrimitiveComponent Object Reference"))
  (`PrimitiveComponent.SetRenderCustomDepth` TouchedComponent false))

(event `self.SPR_buttonmask2.OnBeginCursorOver`
  (params (TouchedComponent :type "PrimitiveComponent Object Reference"))
  (`PrimitiveComponent.SetRenderCustomDepth` TouchedComponent true))

(event `self.SPR_buttonmask2.OnClicked`
  (params (TouchedComponent :type "PrimitiveComponent Object Reference") (ButtonPressed :type "Key Structure"))
  (bind _internalpunchcard (`self.InternalPunchCard`))
  (if (and (`KismetSystemLibrary.IsValid` _internalpunchcard) (< (`KismetStringLibrary.Len` (`/Game/Blueprints/TableObjects/BP_PunchCard.PunchValues` _internalpunchcard)) 8))
    (set `self.LastCharacter` "B")
    (goto _label)))

(event `self.SPR_buttonmask2.OnEndCursorOver`
  (params (TouchedComponent :type "PrimitiveComponent Object Reference"))
  (`PrimitiveComponent.SetRenderCustomDepth` TouchedComponent false))

(event `self.SPR_buttonmask3.OnBeginCursorOver`
  (params (TouchedComponent :type "PrimitiveComponent Object Reference"))
  (`PrimitiveComponent.SetRenderCustomDepth` TouchedComponent true))

(event `self.SPR_buttonmask3.OnClicked`
  (params (TouchedComponent :type "PrimitiveComponent Object Reference") (ButtonPressed :type "Key Structure"))
  (bind _internalpunchcard (`self.InternalPunchCard`))
  (if (and (`KismetSystemLibrary.IsValid` _internalpunchcard) (< (`KismetStringLibrary.Len` (`/Game/Blueprints/TableObjects/BP_PunchCard.PunchValues` _internalpunchcard)) 8))
    (set `self.LastCharacter` "C")
    (goto _label)))

(event `self.SPR_buttonmask3.OnEndCursorOver`
  (params (TouchedComponent :type "PrimitiveComponent Object Reference"))
  (`PrimitiveComponent.SetRenderCustomDepth` TouchedComponent false))

(event `self.SPR_buttonmask4.OnBeginCursorOver`
  (params (TouchedComponent :type "PrimitiveComponent Object Reference"))
  (`PrimitiveComponent.SetRenderCustomDepth` TouchedComponent true))

(event `self.SPR_buttonmask4.OnClicked`
  (params (TouchedComponent :type "PrimitiveComponent Object Reference") (ButtonPressed :type "Key Structure"))
  (bind _internalpunchcard (`self.InternalPunchCard`))
  (if (and (`KismetSystemLibrary.IsValid` _internalpunchcard) (< (`KismetStringLibrary.Len` (`/Game/Blueprints/TableObjects/BP_PunchCard.PunchValues` _internalpunchcard)) 8))
    (set `self.LastCharacter` "D")
    (goto _label)))

(event `self.SPR_buttonmask4.OnEndCursorOver`
  (params (TouchedComponent :type "PrimitiveComponent Object Reference"))
  (`PrimitiveComponent.SetRenderCustomDepth` TouchedComponent false))

(event `self.SPR_buttonmask5.OnBeginCursorOver`
  (params (TouchedComponent :type "PrimitiveComponent Object Reference"))
  (`PrimitiveComponent.SetRenderCustomDepth` TouchedComponent true))

(event `self.SPR_buttonmask5.OnEndCursorOver`
  (params (TouchedComponent :type "PrimitiveComponent Object Reference"))
  (`PrimitiveComponent.SetRenderCustomDepth` TouchedComponent false))

(event `self.SPR_buttonmask5.OnClicked`
  (params (TouchedComponent :type "PrimitiveComponent Object Reference") (ButtonPressed :type "Key Structure"))
  (bind _internalpunchcard (`self.InternalPunchCard`))
  (if (and (`KismetSystemLibrary.IsValid` _internalpunchcard) (< (`KismetStringLibrary.Len` (`/Game/Blueprints/TableObjects/BP_PunchCard.PunchValues` _internalpunchcard)) 8))
    (set `self.LastCharacter` "E")
    (goto _label)))

(event `self.SPR_buttonmask6.OnBeginCursorOver`
  (params (TouchedComponent :type "PrimitiveComponent Object Reference"))
  (`PrimitiveComponent.SetRenderCustomDepth` TouchedComponent true))

(event `self.SPR_buttonmask6.OnEndCursorOver`
  (params (TouchedComponent :type "PrimitiveComponent Object Reference"))
  (`PrimitiveComponent.SetRenderCustomDepth` TouchedComponent false))

(event `self.SPR_buttonmask6.OnClicked`
  (params (TouchedComponent :type "PrimitiveComponent Object Reference") (ButtonPressed :type "Key Structure"))
  (bind _internalpunchcard (`self.InternalPunchCard`))
  (if (and (`KismetSystemLibrary.IsValid` _internalpunchcard) (< (`KismetStringLibrary.Len` (`/Game/Blueprints/TableObjects/BP_PunchCard.PunchValues` _internalpunchcard)) 8))
    (set `self.LastCharacter` "F")
    (goto _label)))

(event `self.SPR_buttonmask7.OnBeginCursorOver`
  (params (TouchedComponent :type "PrimitiveComponent Object Reference"))
  (`PrimitiveComponent.SetRenderCustomDepth` TouchedComponent true))

(event `self.SPR_buttonmask7.OnEndCursorOver`
  (params (TouchedComponent :type "PrimitiveComponent Object Reference"))
  (`PrimitiveComponent.SetRenderCustomDepth` TouchedComponent false))

(event `self.SPR_buttonmask7.OnClicked`
  (params (TouchedComponent :type "PrimitiveComponent Object Reference") (ButtonPressed :type "Key Structure"))
  (bind _internalpunchcard (`self.InternalPunchCard`))
  (if (and (`KismetSystemLibrary.IsValid` _internalpunchcard) (< (`KismetStringLibrary.Len` (`/Game/Blueprints/TableObjects/BP_PunchCard.PunchValues` _internalpunchcard)) 8))
    (set `self.LastCharacter` "G")
    (goto _label)))

(event `self.SPR_buttonmask8.OnBeginCursorOver`
  (params (TouchedComponent :type "PrimitiveComponent Object Reference"))
  (`PrimitiveComponent.SetRenderCustomDepth` TouchedComponent true))

(event `self.SPR_buttonmask8.OnEndCursorOver`
  (params (TouchedComponent :type "PrimitiveComponent Object Reference"))
  (`PrimitiveComponent.SetRenderCustomDepth` TouchedComponent false))

(event `self.SPR_buttonmask8.OnClicked`
  (params (TouchedComponent :type "PrimitiveComponent Object Reference") (ButtonPressed :type "Key Structure"))
  (bind _internalpunchcard (`self.InternalPunchCard`))
  (if (and (`KismetSystemLibrary.IsValid` _internalpunchcard) (< (`KismetStringLibrary.Len` (`/Game/Blueprints/TableObjects/BP_PunchCard.PunchValues` _internalpunchcard)) 8))
    (set `self.LastCharacter` "H")
    (goto _label)))

(event `self.PunchCardSPR.OnClicked`
  (params (TouchedComponent :type "PrimitiveComponent Object Reference") (ButtonPressed :type "Key Structure"))
  (bind _internalpunchcard (`self.InternalPunchCard`))
  (set `/Game/Blueprints/BP_PickupBase.IsHeld` true _internalpunchcard)
  (`SceneComponent.SetVisibility` (`self.PunchCardSPR`) false false)
  (`self.K2_SetActorRelativeLocation` _internalpunchcard (0.0 2000.0 0.0) false true)
  (`/Game/Blueprints/BP_PickupBase.SimulateClick` _internalpunchcard)
  (set `/Game/Blueprints/PlayerStuff/BP_BunkerPlayerPawn.HeldObject` _internalpunchcard (cast `/Game/Blueprints/PlayerStuff/BP_BunkerPlayerPawn` (`Controller.K2_GetPawn` (`GameplayStatics.GetPlayerController` 0)) :!pure true))
  (set `self.InternalPunchCard` null)
  (`TextRenderComponent.K2_SetText` (`self.TextRender`) ""))

(fn `UserConstructionScript`
  (`parent.UserConstructionScript`))