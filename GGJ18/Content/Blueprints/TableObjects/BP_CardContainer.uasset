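; BP_CardContainer is a clickable table object that dispenses punch cards into the player's hand.
; Clicking its PaperSprite spawns a BP_PunchCard, simulates a click on it and sets it as BP_BunkerPlayerPawn's HeldObject.
; The sprite ignores the Camera channel after a click, and a re-armed DoOnce restores blocking when the MyMouse axis reads zero.
; Cursor hover toggles custom depth rendering on the sprite.
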(event `self.PaperSprite.OnClicked`
  (params (TouchedComponent :type "PrimitiveComponent Object Reference") (ButtonPressed :type "Key Structure"))
  (bind _papersprite (`self.PaperSprite`))
  (`|ExecutionSequence`
    (:`then_0`
      (`PrimitiveComponent.SetCollisionResponseToChannel` _papersprite "ECC_Camera" "ECR_Ignore")
      (bind _returnvalue (`|SpawnActorFromClass` "/Game/Blueprints/TableObjects/BP_PunchCard.BP_PunchCard_C" (`KismetMathLibrary.MakeTransform` (0.0 0.0 0.0)) "AlwaysSpawn" "OverrideRootScale" null "" null))
      (`/Game/Blueprints/BP_PickupBase.SimulateClick` _returnvalue)
      (set `/Game/Blueprints/PlayerStuff/BP_BunkerPlayerPawn.HeldObject` _returnvalue (cast `/Game/Blueprints/PlayerStuff/BP_BunkerPlayerPawn` (`Controller.K2_GetPawn` (`GameplayStatics.GetPlayerController` 0)) :!pure true)))
    (:`then_1`
      (goto _label :!via `Reset`))))

(event `InputAxis|MyMouse` :consume false
  (params (AxisValue :type "Float (single-precision)"))
  (if (== AxisValue 0.0)
    (`/Engine/EditorBlueprintResources/StandardMacros.DoOnce` true :!label _label
      (:`Completed`
        (`PrimitiveComponent.SetCollisionResponseToChannel` (`self.PaperSprite`) "ECC_Camera" "ECR_Block")))))

(event `self.PaperSprite.OnBeginCursorOver`
  (params (TouchedComponent :type "PrimitiveComponent Object Reference"))
  (`PrimitiveComponent.SetRenderCustomDepth` TouchedComponent true))

(event `self.PaperSprite.OnEndCursorOver`
  (params (TouchedComponent :type "PrimitiveComponent Object Reference"))
  (`PrimitiveComponent.SetRenderCustomDepth` TouchedComponent false))

(fn `UserConstructionScript`)