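; BP_ThrashArea is a table object that disposes of the punch card the player is holding.
; On DoInteraction, it gets player controller 0's BP_BunkerPlayerPawn, casts its HeldObject to BP_PunchCard and destroys that actor.
; It does not explicitly clear the pawn's HeldObject reference, and other held object types are not handled.
; BeginPlay, overlap and Tick are unused placeholders.
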(event `self.DoInteraction`
  (`self.K2_DestroyActor` (cast `/Game/Blueprints/TableObjects/BP_PunchCard` (`/Game/Blueprints/PlayerStuff/BP_BunkerPlayerPawn.HeldObject` (cast `/Game/Blueprints/PlayerStuff/BP_BunkerPlayerPawn` (`Controller.K2_GetPawn` (`GameplayStatics.GetPlayerController` 0)) :!pure true)) :!pure true)))

(fn `UserConstructionScript`
  (`parent.UserConstructionScript`))