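; Player pawn for the bunker view that pans the camera across the X-Z plane by mouse edge-scrolling and directional input.
; Tick nudges CamOffset when the cursor enters the viewport-edge deadzone, and Gates opened by held inputs pass Tick through for the same nudge.
; AddToOffset clamps the offset to MaxCamOffsets, then Tick teleports the pawn there.
; Steps are fixed per frame, so pan speed depends on framerate.
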(event `InputAction|Left`
  (params (Key :type "Key Structure"))
  ;[1 1 1] Keyboard input for camera
  (:`Pressed`
    (goto _label :!via `Open`))
  (:`Released`
    (goto _label :!via `Close`)))

(event `self.ReceiveTick`
  (params (DeltaSeconds :type "Float (single-precision)"))
  (bind (_camoffset_x _camoffset_y) (`KismetMathLibrary.BreakVector2D` (`self.CamOffset`)))
  (bind (_x _y) (`KismetMathLibrary.BreakVector2D` (`self.WindowDeadzone`)))
  (bind (_x_2 _y_2) (`KismetMathLibrary.BreakVector2D` (/ (`WidgetLayoutLibrary.GetViewportSize`) (`WidgetLayoutLibrary.GetViewportScale`))))
  ;[1 1 1] Mouse Panning
  (bind _returnvalue (`WidgetLayoutLibrary.GetMousePositionOnViewport`))
  (bind (_x_3 _y_3) (`KismetMathLibrary.BreakVector2D` _returnvalue))
  (if (<= _x_3 _x)
    (`self.AddToOffset` -5.0
      (:`Out`
        _))
    (elif (>= _x_3 (- _x_2 _x))
      (`self.AddToOffset` 5.0
        (:`Out`
          _))))
  (if (<= _y_3 _y)
    (`self.AddToOffset` 0.0 5.0
      (:`Out`
        _))
    (elif (>= _y_3 (- _y_2 _y))
      (`self.AddToOffset` 0.0 -5.0
        (:`Out`
          _))))
  (`|ExecutionSequence`
    (:`then_0`
      ;[1 1 1] Keyboard input for camera
      (`/Engine/EditorBlueprintResources/StandardMacros.Gate` true :!label _label
        (:`Exit`
          (`self.AddToOffset` -5.0))))
    (:`then_1`
      (`/Engine/EditorBlueprintResources/StandardMacros.Gate` true :!label _label_2
        (:`Exit`
          (`self.AddToOffset` 5.0))))
    (:`then_2`
      (`/Engine/EditorBlueprintResources/StandardMacros.Gate` true :!label _label_3
        (:`Exit`
          (`self.AddToOffset` 0.0 5.0))))
    (:`then_3`
      (`/Engine/EditorBlueprintResources/StandardMacros.Gate` true :!label _label_4
        (:`Exit`
          (`self.AddToOffset` 0.0 -5.0))))
    (:`then_4`
      (`self.K2_SetActorLocation` (`KismetMathLibrary.MakeVector` _camoffset_x 0.0 _camoffset_y) false true))))

(event `InputAction|Right`
  (params (Key :type "Key Structure"))
  ;[1 1 1] Keyboard input for camera
  (:`Pressed`
    (goto _label_2 :!via `Open`))
  (:`Released`
    (goto _label_2 :!via `Close`)))

(event `InputAction|Up`
  (params (Key :type "Key Structure"))
  ;[1 1 1] Keyboard input for camera
  (:`Pressed`
    (goto _label_3 :!via `Open`))
  (:`Released`
    (goto _label_3 :!via `Close`)))

(event `InputAction|Down`
  (params (Key :type "Key Structure"))
  ;[1 1 1] Keyboard input for camera
  (:`Pressed`
    (goto _label_4 :!via `Open`))
  (:`Released`
    (goto _label_4 :!via `Close`)))

(fn `UserConstructionScript`)