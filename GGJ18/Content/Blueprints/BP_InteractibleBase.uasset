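; Base interactible sprite actor that accepts a specific kind of object held by the bunker player pawn.
; CheckHoldingObject compares the held object's class to one selected by InteractibleType; only PunchCard has a class assigned.
; A match enables a custom-depth highlight on hover and calls the empty DoInteraction hook on release over the sprite.
; The MyMouse axis toggles the sprite's Camera-channel collision, blocking only while it reads 1.
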(event `self.Sprite.OnBeginCursorOver`
  (params (TouchedComponent :type "PrimitiveComponent Object Reference"))
  (`self.CheckHoldingObject`
    (:`True`
      (`PrimitiveComponent.SetRenderCustomDepth` TouchedComponent true))))

(event `self.Sprite.OnEndCursorOver`
  (params (TouchedComponent :type "PrimitiveComponent Object Reference"))
  (`PrimitiveComponent.SetRenderCustomDepth` TouchedComponent false))

(event `self.Sprite.OnReleased`
  (params (TouchedComponent :type "PrimitiveComponent Object Reference") (ButtonReleased :type "Key Structure"))
  (`self.CheckHoldingObject`
    (:`True`
      (`self.DoInteraction`))))

(event `DoInteraction`)

(event `InputAxis|MyMouse` :consume false
  (params (AxisValue :type "Float (single-precision)"))
  (bind _sprite (`self.Sprite`))
  (if (== AxisValue 1.0)
    (`PrimitiveComponent.SetCollisionResponseToChannel` _sprite "ECC_Camera" "ECR_Block")
    (else
      (`PrimitiveComponent.SetCollisionResponseToChannel` _sprite "ECC_Camera" "ECR_Ignore"))))

(fn `UserConstructionScript`)