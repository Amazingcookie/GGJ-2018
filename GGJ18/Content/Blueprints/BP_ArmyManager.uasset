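; Army manager actor that creates squads of infantry, cavalry, tanks and artillery and tracks those deployed.
; SpawnSquadAt spawns a BP_Squad data actor, stores its array index as SquadID, then sets its node location and unit counts.
; BeginPlay caches the first BP_NodeManager found.
; Space spawns a hardcoded squad at the default node, and Enter moves the first squad to TempTarget.
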(event `self.ReceiveBeginPlay`
  (bind _outactors (`GameplayStatics.GetAllActorsOfClass` "/Game/Blueprints/BP_NodeManager.BP_NodeManager_C"))
  (for _array_element _outactors
    (set `self.NodeManager` _array_element)
    (break)))

(event `Key|SpaceBar`
  (params (Key :type "Key Structure"))
  (:`Pressed`
    (`self.SpawnSquadAt` (`self.Default Spawn Node`) 300 200 100 100)))

(event `Key|Enter`
  (params (Key :type "Key Structure"))
  (:`Pressed`
    (bind _returnedsquad (`self.GetSquadAtIndex` 0))
    (`/Game/Blueprints/BP_Squad.MoveTo` _returnedsquad (`self.TempTarget`))))

(fn `GetSquadAtIndex`
  (params (Index :type Integer))
  (returns (ReturnedSquad :type "/Game/Blueprints/BP_Squad Object Reference"))
  (for (_array_element _array_index) (`self.Deployed Squads`)
    (if (== Index _array_index)
      (return _array_element))))

(fn `SpawnSquadAt`
  (params (SpawnNode :type "/Game/Blueprints/BP_Node Object Reference") (Infantry :type Integer) (Cavalry :type Integer) (Tanks :type Integer) (Artillery :type Integer))
  (`|ExecutionSequence`
    (:`then_0`
      ;[1 1 1] Creates a new actor to hold the data for us
      (bind _returnvalue (`|SpawnActorFromClass` "/Game/Blueprints/BP_Squad.BP_Squad_C" (`SceneComponent.K2_GetComponentToWorld` (`self.DefaultSceneRoot`)) "AlwaysSpawn" "OverrideRootScale" null null))
      ;[1 1 1] Add the squad to the array, and store its id
      (bind _returnvalue_2 (`KismetArrayLibrary.Array_Add` (`self.Deployed Squads`) _returnvalue))
      (set `/Game/Blueprints/BP_Squad.SquadID` _returnvalue_2 _returnvalue))
    (:`then_1`
      ;[1 1 1] Spawn the squad at the designated position
      (set `/Game/Blueprints/BP_Squad.Current Location` SpawnNode _returnvalue)
      ;[1 1 1] Setting the proper amount of units as specifeid
      (set `/Game/Blueprints/BP_Squad.Infantry` Infantry _returnvalue)
      (set `/Game/Blueprints/BP_Squad.Cavalry` Cavalry _returnvalue)
      (set `/Game/Blueprints/BP_Squad.Tanks` Tanks _returnvalue)
      (set `/Game/Blueprints/BP_Squad.Artillery` Artillery _returnvalue))))

(fn `UserConstructionScript`)